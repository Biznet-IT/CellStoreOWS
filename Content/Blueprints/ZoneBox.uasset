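; ZoneBox is a trigger actor that shows a catalogue of items in the player's UI when its Box is overlapped.
; On overlap it blocks player 0's OWSNewPawn movement, shows the UI and copies its item lists into the WidgDocJumbo widget, then refreshes button images.
; When an actor overlap ends, it clears the widget's grid panel.
; Both events act on player pawn 0, regardless of which actor overlaps.
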(event OnComponentBeginOverlap(Box)
  (params (OverlappedComponent :type Primitive%20Component%20Object%20Reference) (OtherActor :type Actor%20Object%20Reference) (OtherComp :type Primitive%20Component%20Object%20Reference) (OtherBodyIndex :type Integer) (bFromSweep :type Boolean) (SweepResult :type Hit%20Result%20Structure%20%28by%20ref%29))
  (bind _asowsnew_pawn (Utilities|Casting|CastToOWSNewPawn (Game|Player|GetPlayerPawn 0)))
  (Default|BlockMovementandShowUi _asowsnew_pawn)
  (Variables|/Game/Blueprints/WidgDocProductListJumbo.WidgDocProductListJumbo_C|SetButtonsNames (Variables|/Game/ThirdPersonBP/Blueprints/OWSNewPawn.OWSNewPawn_C|GetWidgDocJumbo _asowsnew_pawn) (Variables|Items|GetListOfItemsNames))
  (Variables|/Game/Blueprints/WidgDocProductListJumbo.WidgDocProductListJumbo_C|SetButtonsImages (Variables|/Game/ThirdPersonBP/Blueprints/OWSNewPawn.OWSNewPawn_C|GetWidgDocJumbo _asowsnew_pawn) (Variables|Items|GetListOfItemTexture2D))
  (Variables|/Game/Blueprints/WidgDocProductListJumbo.WidgDocProductListJumbo_C|SetButtonsPrices (Variables|/Game/ThirdPersonBP/Blueprints/OWSNewPawn.OWSNewPawn_C|GetWidgDocJumbo _asowsnew_pawn) (Variables|Items|GetListOfItemPrices))
  (Variables|/Game/Blueprints/WidgDocProductListJumbo.WidgDocProductListJumbo_C|SetButtonsStock (Variables|/Game/ThirdPersonBP/Blueprints/OWSNewPawn.OWSNewPawn_C|GetWidgDocJumbo _asowsnew_pawn) (Variables|Items|GetListOfItemStock))
  (Variables|/Game/Blueprints/WidgDocProductListJumbo.WidgDocProductListJumbo_C|SetButtonsExternalLinks (Variables|/Game/ThirdPersonBP/Blueprints/OWSNewPawn.OWSNewPawn_C|GetWidgDocJumbo _asowsnew_pawn) (Variables|Items|GetListOfItemsExternalLinks))
  (Variables|/Game/Blueprints/WidgDocProductListJumbo.WidgDocProductListJumbo_C|SetButtonsSimillarItems (Variables|/Game/ThirdPersonBP/Blueprints/OWSNewPawn.OWSNewPawn_C|GetWidgDocJumbo _asowsnew_pawn) (Variables|Items|GetListOfItemsSimilarItems))
  (Default|HandleBrushImages (Variables|/Game/ThirdPersonBP/Blueprints/OWSNewPawn.OWSNewPawn_C|GetWidgDocJumbo _asowsnew_pawn)))

(event Collision|EventActorBeginOverlap
  (params (OtherActor :type Actor%20Object%20Reference)))

(event EventTick
  (params (DeltaSeconds :type Float%20%28single-precision%29)))

(event Collision|EventActorEndOverlap
  (params (OtherActor :type Actor%20Object%20Reference))
  (bind _asowsnew_pawn (Utilities|Casting|CastToOWSNewPawn (Game|Player|GetPlayerPawn 0)))
  (Widget|Panel|ClearChildren (Variables|/Game/Blueprints/WidgDocProductListJumbo.WidgDocProductListJumbo_C|GetGridPanel_149 (Variables|/Game/ThirdPersonBP/Blueprints/OWSNewPawn.OWSNewPawn_C|GetWidgDocJumbo _asowsnew_pawn))))

(fn ConstructionScript)