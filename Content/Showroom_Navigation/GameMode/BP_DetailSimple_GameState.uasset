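; Game state for the showroom's simple detail view, setting up the player's pawn and menu when play begins.
; BeginPlay clears existing widgets, possesses the BP_FocusPawn_simple found in the level and adds a WBP_FocusPointSimple menu to the viewport.
; It binds the menu's Go Home and Home-and-Reset dispatchers and re-broadcasts them through its own bridge dispatchers.
; A game instance cast leading into the setup is left unconnected.
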(event Custom|CustomEvent_0
  ;[1 1 1] Button Home
  (Default|CallDispatcherBridge))

(event Custom|Home_and_reset
  ;[1 1 1] Button Back
  (Default|CallEventDispatcherHomeandResetBridge))

(event EventBeginPlay
  (bind _returnvalue (Game|GetPlayerController 0))
  ;[1 1 1] Posses Simple Pawn and Menue
  (Viewport|RemoveAllWidgets)
  (bind _returnvalue_2 (Actor|GetActorOfClass "/Game/Showroom_Navigation/Blueprint/FocusPoint_Simple/BP_FocusPawn_simple.BP_FocusPawn_simple_C"))
  (Pawn|Possess _returnvalue _returnvalue_2)
  (bind _returnvalue_3 (UserInterface|CreateWidget "/Game/Showroom_Navigation/Blueprint/UI_Widget/WBP_FocusPointSimple.WBP_FocusPointSimple_C" _returnvalue))
  (UserInterface|Viewport|AddtoViewport _returnvalue_3 0)
  (Utilities|FlowControl|Sequence
    (:then_0
      ;[1 1 1] Button Home
      (bind _foundwidgets (Widget|GetAllWidgetsOfClass "/Game/Showroom_Navigation/Blueprint/UI_Widget/WBP_FocusPointSimple.WBP_FocusPointSimple_C" true))
      (EventDispatchers|BindEventtoNewEventDispatcherGoHome _foundwidgets (delegate Custom|CustomEvent_0)))
    (:then_1
      ;[1 1 1] Button Back
      (bind _foundwidgets_2 (Widget|GetAllWidgetsOfClass "/Game/Showroom_Navigation/Blueprint/UI_Widget/WBP_FocusPointSimple.WBP_FocusPointSimple_C" true))
      (EventDispatchers|BindEventtoEventDispatcherHomeandReset _foundwidgets_2 (delegate Custom|Home_and_reset)))))

(fn ConstructionScript)