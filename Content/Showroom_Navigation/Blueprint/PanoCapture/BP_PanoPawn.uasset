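; Pawn that batch-captures panoramic screenshots at navigation points in the showroom level.
; BeginPlay hides PanoHide-tagged actors, then a one-time pass takes a manual list or gathers PanoIndex, Waypoint and ZoomPoint actors, with optional exclusions.
; Delayed Tick, or key 7 in manual mode, steps backwards through the list, placing the camera by point type and height offset, ending on the base target.
; Each stop runs SP.PanoramicScreenshot when ActivateCapture is on.
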(event EventTick
  (params (DeltaSeconds :type Float%20%28single-precision%29))
  (Utilities|FlowControl|Delay 0.6)
  (if (not (Variables|Default|GetDISABLE))
    ;[1 1 1] Automaic or Key
    (if (not (Variables|Default|GetGo_by_Key%207))
      (Utilities|FlowControl|Sequence
        (:then_0
          (if (Variables|Default|GetCaptureByList)
            ;[1 1 1] capture by list
            (Utilities|FlowControl|DoOnce false
              (:Completed
                (bind _output_get (Variables|Default|SetAll_Capture (Variables|Default|GetList%20Panos)))
                (Variables|Default|SetValue_execute (Utilities|Array|Length _output_get))
                (Transformation|SetWorldLocation (Variables|Default|GetCamera) "0, 0, 0" false false)))
            (else
              (Utilities|FlowControl|DoOnce false
                (:Completed
                  ;[1 1 1] Get all Pointsand create Arrays
                  (bind _outactors (Actor|GetAllActorswithTag "ZoomPoint"))
                  (bind _outactors_2 (Actor|GetAllActorswithTag "Waypoint"))
                  (bind _outactors_3 (Actor|GetAllActorswithTag "PanoIndex"))
                  (Utilities|Array|AppendArray _outactors_2 _outactors)
                  (Utilities|Array|Insert _outactors_2 (Utilities|Array|Get(acopy) _outactors_3))
                  (if (Variables|Default|GetRemove_from_List)
                    (for _array_element (Variables|Default|GetRemove_Panos)
                      (Utilities|Array|RemoveItem _outactors_2 _array_element)
                      (bind _output_get_2 (Variables|Default|SetAll_Capture _outactors_2))
                      (Variables|Default|SetValue_execute (Utilities|Array|Length _output_get_2))
                      (Transformation|SetWorldLocation (Variables|Default|GetCamera) "0, 0, 0" false false))
                    (else
                      (bind _output_get_3 (Variables|Default|SetAll_Capture _outactors_2))
                      (Variables|Default|SetValue_execute (Utilities|Array|Length _output_get_3))
                      (Transformation|SetWorldLocation (Variables|Default|GetCamera) "0, 0, 0" false false))))))))
        (:then_1
          ;[1 1 1] Print "All Done" when finished
          (if (== (Variables|Default|GetValue_execute) 0)
            (Development|PrintString "ALL Done")
            (else
              ;[1 1 1] Decremend
              (bind _result (Math|Integer|DecrementInt (Variables|Default|GetValue_execute))
                (:%20%20
                  ;[1 1 1] check if Base Target
                  (bind _output_get_4 (Variables|Default|SetValue_execute _result))
                  (if (== _output_get_4 0)
                    ;[1 1 1] Use Pase Target Center Position
                    (if (Variables|Default|GetBaseTarget%20center%20position)
                      (Transformation|SetWorldLocation (Variables|Default|GetCamera) (Math|Vector|MakeVector (.x (Transformation|GetActorLocation (Utilities|Array|Get(acopy) (Variables|Default|GetAll_Capture)))) (.y (Transformation|GetActorLocation (Utilities|Array|Get(acopy) (Variables|Default|GetAll_Capture)))) (+ (.z (Transformation|GetActorLocation (Utilities|Array|Get(acopy) (Variables|Default|GetAll_Capture)))) (Variables|Default|GetBaseTarget_CameraHeight))) false false)
                      (if (Variables|Default|GetActivate_Capture)
                        (Development|ExecuteConsoleCommand "SP.PanoramicScreenshot" 0))
                      (else
                        ;[1 1 1] Use BaseTarget Camera Position
                        (Transformation|SetWorldTransform (Variables|Default|GetCamera) (Math|Transform|MakeTransform (Math|Vector|MakeVector (.x (.location (Transformation|GetWorldTransform (Actor|GetComponentbyClass (Utilities|Array|Get(acopy) (Variables|Default|GetAll_Capture)) "/Script/Engine.CameraComponent")))) (.y (.location (Transformation|GetWorldTransform (Actor|GetComponentbyClass (Utilities|Array|Get(acopy) (Variables|Default|GetAll_Capture)) "/Script/Engine.CameraComponent")))) (.z (.location (Transformation|GetWorldTransform (Actor|GetComponentbyClass (Utilities|Array|Get(acopy) (Variables|Default|GetAll_Capture)) "/Script/Engine.CameraComponent"))))) (.rotation (Transformation|GetWorldTransform (Actor|GetComponentbyClass (Utilities|Array|Get(acopy) (Variables|Default|GetAll_Capture)) "/Script/Engine.CameraComponent"))) "1.000000,1.000000,1.000000") false false)
                        (Transformation|AddLocalOffset (Variables|Default|GetCamera) (Math|Vector|MakeVector (Variables|Default|GetBaseTarget-ZoomIn) 0.0 0.0) false false)
                        (if (Variables|Default|GetActivate_Capture)
                          (Development|ExecuteConsoleCommand "SP.PanoramicScreenshot" 0))))
                    (elif (Actor|ActorHasTag (Utilities|Array|Get(acopy) (Variables|Default|GetAll_Capture) _output_get_4) "ZoomPoint")
                      (if (Variables|Default|GetZoomPoint%20center%20position)
                        ;[1 1 1] Capture Zoom Point center Position
                        (Transformation|SetWorldLocation (Variables|Default|GetCamera) (Math|Vector|MakeVector (.x (Transformation|GetActorLocation (Utilities|Array|Get(acopy) (Variables|Default|GetAll_Capture) _result))) (.y (Transformation|GetActorLocation (Utilities|Array|Get(acopy) (Variables|Default|GetAll_Capture) _result))) (+ (.z (Transformation|GetActorLocation (Utilities|Array|Get(acopy) (Variables|Default|GetAll_Capture) _result))) (Variables|Default|GetZoomPoint_CameraHeight))) false false)
                        (if (Variables|Default|GetActivate_Capture)
                          (Development|ExecuteConsoleCommand "SP.PanoramicScreenshot" 0))
                        (else
                          ;[1 1 1] capture ZoomPoint from PanoPoint
                          (bind _asbp_zoom_target (Utilities|Casting|CastToBP_ZoomTarget (Utilities|Array|Get(acopy) (Variables|Default|GetAll_Capture) _output_get_4)))
                          (Transformation|SetWorldLocation (Variables|Default|GetCamera) (Math|Vector|MakeVector (.x (Transformation|GetWorldLocation (Variables|/Game/Showroom_Navigation/Blueprint/BP_ZoomTarget.BP_ZoomTarget_C|GetPanoPoint _asbp_zoom_target))) (.y (Transformation|GetWorldLocation (Variables|/Game/Showroom_Navigation/Blueprint/BP_ZoomTarget.BP_ZoomTarget_C|GetPanoPoint _asbp_zoom_target))) (+ (.z (Transformation|GetWorldLocation (Variables|/Game/Showroom_Navigation/Blueprint/BP_ZoomTarget.BP_ZoomTarget_C|GetPanoPoint _asbp_zoom_target))) (Variables|Default|GetZoomPoint_CameraHeight))) false false)
                          (if (Variables|Default|GetActivate_Capture)
                            (Development|ExecuteConsoleCommand "SP.PanoramicScreenshot" 0))))
                      (else
                        ;[1 1 1] capture Waypoint
                        (Transformation|SetWorldLocation (Variables|Default|GetCamera) (Math|Vector|MakeVector (.x (Transformation|GetActorLocation (Utilities|Array|Get(acopy) (Variables|Default|GetAll_Capture) _result))) (.y (Transformation|GetActorLocation (Utilities|Array|Get(acopy) (Variables|Default|GetAll_Capture) _result))) (+ (.z (Transformation|GetActorLocation (Utilities|Array|Get(acopy) (Variables|Default|GetAll_Capture) _result))) (Variables|Default|GetWaypoint_CameraHeight))) false false)
                        (if (Variables|Default|GetActivate_Capture)
                          (Development|ExecuteConsoleCommand "SP.PanoramicScreenshot" 0))))))))))))))

(event EventBeginPlay
  ;[1 1 1] Set input Mode
  (if (not (Variables|Default|GetDISABLE))
    (Input|SetInputModeGameOnly (Game|GetPlayerController 0) false)
    ;[1 1 1] Hide UI - and Objects with Tag PanoHide
    (Utilities|FlowControl|Delay 0.4)
    (bind _outactors (Actor|GetAllActorswithTag "PanoHide"))
    (for _array_element _outactors
      (Rendering|SetActorHiddenInGame _array_element true))))

(event Input|KeyboardEvents|7
  (params (Key :type Key%20Structure))
  ;[1 1 1] Automaic or Key
  (:Pressed
    (if (not (Variables|Default|GetDISABLE))
      (Utilities|FlowControl|Sequence
        (:then_0
          (if (Variables|Default|GetCaptureByList)
            ;[1 1 1] capture by list
            (Utilities|FlowControl|DoOnce false
              (:Completed
                (bind _output_get (Variables|Default|SetAll_Capture (Variables|Default|GetList%20Panos)))
                (Variables|Default|SetValue_execute (Utilities|Array|Length _output_get))
                (Transformation|SetWorldLocation (Variables|Default|GetCamera) "0, 0, 0" false false)))
            (else
              (Utilities|FlowControl|DoOnce false
                (:Completed
                  ;[1 1 1] Get all Pointsand create Arrays
                  (bind _outactors (Actor|GetAllActorswithTag "ZoomPoint"))
                  (bind _outactors_2 (Actor|GetAllActorswithTag "Waypoint"))
                  (bind _outactors_3 (Actor|GetAllActorswithTag "PanoIndex"))
                  (Utilities|Array|AppendArray _outactors_2 _outactors)
                  (Utilities|Array|Insert _outactors_2 (Utilities|Array|Get(acopy) _outactors_3))
                  (if (Variables|Default|GetRemove_from_List)
                    (for _array_element (Variables|Default|GetRemove_Panos)
                      (Utilities|Array|RemoveItem _outactors_2 _array_element)
                      (bind _output_get_2 (Variables|Default|SetAll_Capture _outactors_2))
                      (Variables|Default|SetValue_execute (Utilities|Array|Length _output_get_2))
                      (Transformation|SetWorldLocation (Variables|Default|GetCamera) "0, 0, 0" false false))
                    (else
                      (bind _output_get_3 (Variables|Default|SetAll_Capture _outactors_2))
                      (Variables|Default|SetValue_execute (Utilities|Array|Length _output_get_3))
                      (Transformation|SetWorldLocation (Variables|Default|GetCamera) "0, 0, 0" false false))))))))
        (:then_1
          ;[1 1 1] Print "All Done" when finished
          (if (== (Variables|Default|GetValue_execute) 0)
            (Development|PrintString "ALL Done")
            (else
              ;[1 1 1] Decremend
              (bind _result (Math|Integer|DecrementInt (Variables|Default|GetValue_execute))
                (:%20%20
                  ;[1 1 1] check if Base Target
                  (bind _output_get_4 (Variables|Default|SetValue_execute _result))
                  (if (== _output_get_4 0)
                    ;[1 1 1] Use Pase Target Center Position
                    (if (Variables|Default|GetBaseTarget%20center%20position)
                      (Transformation|SetWorldLocation (Variables|Default|GetCamera) (Math|Vector|MakeVector (.x (Transformation|GetActorLocation (Utilities|Array|Get(acopy) (Variables|Default|GetAll_Capture)))) (.y (Transformation|GetActorLocation (Utilities|Array|Get(acopy) (Variables|Default|GetAll_Capture)))) (+ (.z (Transformation|GetActorLocation (Utilities|Array|Get(acopy) (Variables|Default|GetAll_Capture)))) (Variables|Default|GetBaseTarget_CameraHeight))) false false)
                      (if (Variables|Default|GetActivate_Capture)
                        (Development|ExecuteConsoleCommand "SP.PanoramicScreenshot" 0))
                      (else
                        ;[1 1 1] Use BaseTarget Camera Position
                        (Transformation|SetWorldTransform (Variables|Default|GetCamera) (Math|Transform|MakeTransform (Math|Vector|MakeVector (.x (.location (Transformation|GetWorldTransform (Actor|GetComponentbyClass (Utilities|Array|Get(acopy) (Variables|Default|GetAll_Capture)) "/Script/Engine.CameraComponent")))) (.y (.location (Transformation|GetWorldTransform (Actor|GetComponentbyClass (Utilities|Array|Get(acopy) (Variables|Default|GetAll_Capture)) "/Script/Engine.CameraComponent")))) (.z (.location (Transformation|GetWorldTransform (Actor|GetComponentbyClass (Utilities|Array|Get(acopy) (Variables|Default|GetAll_Capture)) "/Script/Engine.CameraComponent"))))) (.rotation (Transformation|GetWorldTransform (Actor|GetComponentbyClass (Utilities|Array|Get(acopy) (Variables|Default|GetAll_Capture)) "/Script/Engine.CameraComponent"))) "1.000000,1.000000,1.000000") false false)
                        (Transformation|AddLocalOffset (Variables|Default|GetCamera) (Math|Vector|MakeVector (Variables|Default|GetBaseTarget-ZoomIn) 0.0 0.0) false false)
                        (if (Variables|Default|GetActivate_Capture)
                          (Development|ExecuteConsoleCommand "SP.PanoramicScreenshot" 0))))
                    (elif (Actor|ActorHasTag (Utilities|Array|Get(acopy) (Variables|Default|GetAll_Capture) _output_get_4) "ZoomPoint")
                      (if (Variables|Default|GetZoomPoint%20center%20position)
                        ;[1 1 1] Capture Zoom Point center Position
                        (Transformation|SetWorldLocation (Variables|Default|GetCamera) (Math|Vector|MakeVector (.x (Transformation|GetActorLocation (Utilities|Array|Get(acopy) (Variables|Default|GetAll_Capture) _result))) (.y (Transformation|GetActorLocation (Utilities|Array|Get(acopy) (Variables|Default|GetAll_Capture) _result))) (+ (.z (Transformation|GetActorLocation (Utilities|Array|Get(acopy) (Variables|Default|GetAll_Capture) _result))) (Variables|Default|GetZoomPoint_CameraHeight))) false false)
                        (if (Variables|Default|GetActivate_Capture)
                          (Development|ExecuteConsoleCommand "SP.PanoramicScreenshot" 0))
                        (else
                          ;[1 1 1] capture ZoomPoint from PanoPoint
                          (bind _asbp_zoom_target (Utilities|Casting|CastToBP_ZoomTarget (Utilities|Array|Get(acopy) (Variables|Default|GetAll_Capture) _output_get_4)))
                          (Transformation|SetWorldLocation (Variables|Default|GetCamera) (Math|Vector|MakeVector (.x (Transformation|GetWorldLocation (Variables|/Game/Showroom_Navigation/Blueprint/BP_ZoomTarget.BP_ZoomTarget_C|GetPanoPoint _asbp_zoom_target))) (.y (Transformation|GetWorldLocation (Variables|/Game/Showroom_Navigation/Blueprint/BP_ZoomTarget.BP_ZoomTarget_C|GetPanoPoint _asbp_zoom_target))) (+ (.z (Transformation|GetWorldLocation (Variables|/Game/Showroom_Navigation/Blueprint/BP_ZoomTarget.BP_ZoomTarget_C|GetPanoPoint _asbp_zoom_target))) (Variables|Default|GetZoomPoint_CameraHeight))) false false)
                          (if (Variables|Default|GetActivate_Capture)
                            (Development|ExecuteConsoleCommand "SP.PanoramicScreenshot" 0))))
                      (else
                        ;[1 1 1] capture Waypoint
                        (Transformation|SetWorldLocation (Variables|Default|GetCamera) (Math|Vector|MakeVector (.x (Transformation|GetActorLocation (Utilities|Array|Get(acopy) (Variables|Default|GetAll_Capture) _result))) (.y (Transformation|GetActorLocation (Utilities|Array|Get(acopy) (Variables|Default|GetAll_Capture) _result))) (+ (.z (Transformation|GetActorLocation (Utilities|Array|Get(acopy) (Variables|Default|GetAll_Capture) _result))) (Variables|Default|GetWaypoint_CameraHeight))) false false)
                        (if (Variables|Default|GetActivate_Capture)
                          (Development|ExecuteConsoleCommand "SP.PanoramicScreenshot" 0))))))))))))))

(fn ConstructionScript)