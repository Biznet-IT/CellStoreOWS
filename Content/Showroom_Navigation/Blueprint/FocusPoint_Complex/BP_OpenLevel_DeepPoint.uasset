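; BP_OpenLevel_DeepPoint is a clickable billboard hotspot in the showroom that opens the level named in LevelToGo.
; Touch release (ignored while the touch is moving) or click (ignored on first touch) flags deep level in the GameInstance.
; It also saves the focus pawn's spring arm and root transforms there before switching levels.
; The construction script sizes the button and optional label, which turns toward the camera on Tick.
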(event OnInputTouchEnd(Box_Trigger)
  (params (FingerIndex :type ETouchIndex%20Enum :default "Touch1") (TouchedComponent :type Primitive%20Component%20Object%20Reference))
  (bind _returnvalue (Game|GetGameInstance))
  ;[1 1 1] Do not click when Touc is moving
  (bind _asbp_gameinstance_showroom (Utilities|Casting|CastToBP_Gameinstance_showroom (Game|GetGameInstance)))
  (if (not (Variables|/Game/Showroom_Navigation/Gameinstance/BP_Gameinstance_showroom.BP_Gameinstance_showroom_C|Getis_Touch_moving _asbp_gameinstance_showroom))
    ;[1 1 1] Set deepLevel on
    (bind _asbp_gameinstance_showroom_2 (Utilities|Casting|CastToBP_Gameinstance_showroom _returnvalue))
    (Variables|/Game/Showroom_Navigation/Gameinstance/BP_Gameinstance_showroom.BP_Gameinstance_showroom_C|SetIs_deep_Level _asbp_gameinstance_showroom_2 true)
    (bind _asbp_gameinstance_showroom_3 (Utilities|Casting|CastToBP_Gameinstance_showroom _returnvalue))
    ;[1 1 1] Get Transforms from Pawn
    (bind _asbp_focus_pawn_complex (Utilities|Casting|CastToBP_FocusPawnComplex (Game|Player|GetPlayerPawn 0)))
    ;[1 1 1] Save Transforms LevelSwitch
    (Variables|/Game/Showroom_Navigation/Gameinstance/BP_Gameinstance_showroom.BP_Gameinstance_showroom_C|SetGI_ArmLocation_LevelSwitch_DeepP _asbp_gameinstance_showroom_3 (Transformation|GetWorldLocation (Variables|/Game/Showroom_Navigation/Blueprint/FocusPoint_Complex/BP_FocusPawnComplex.BP_FocusPawnComplex_C|GetSpringArm _asbp_focus_pawn_complex)))
    (Variables|/Game/Showroom_Navigation/Gameinstance/BP_Gameinstance_showroom.BP_Gameinstance_showroom_C|SetGI_ArmLength_LevelSwitch_DeepP _asbp_gameinstance_showroom_3 (Variables|/Script/Engine.SpringArmComponent|GetTargetArmLength (Variables|/Game/Showroom_Navigation/Blueprint/FocusPoint_Complex/BP_FocusPawnComplex.BP_FocusPawnComplex_C|GetSpringArm _asbp_focus_pawn_complex)))
    (Variables|/Game/Showroom_Navigation/Gameinstance/BP_Gameinstance_showroom.BP_Gameinstance_showroom_C|SetGI_ArmRotation_LevelSwitch_DeepP _asbp_gameinstance_showroom_3 (Class|SpringArmComponent|GetTargetRotation (Variables|/Game/Showroom_Navigation/Blueprint/FocusPoint_Complex/BP_FocusPawnComplex.BP_FocusPawnComplex_C|GetSpringArm _asbp_focus_pawn_complex)))
    (Variables|/Game/Showroom_Navigation/Gameinstance/BP_Gameinstance_showroom.BP_Gameinstance_showroom_C|SetGI_DefaultSceneRoot_LevelSwitch_DeepP _asbp_gameinstance_showroom_3 (.location (Transformation|GetActorTransform _asbp_focus_pawn_complex)))
    ;[1 1 1] Open Level
    (Game|OpenLevel(byName) (Variables|Default|GetLevelToGo))))

(event OnClicked(Box_Trigger)
  (params (TouchedComponent :type Primitive%20Component%20Object%20Reference) (ButtonPressed :type Key%20Structure))
  (bind _returnvalue (Game|GetGameInstance))
  ;[1 1 1] Do not click when Touc is moving
  (bind _asbp_gameinstance_showroom (Utilities|Casting|CastToBP_Gameinstance_showroom (Game|GetGameInstance)))
  (if (not (Variables|/Game/Showroom_Navigation/Gameinstance/BP_Gameinstance_showroom.BP_Gameinstance_showroom_C|Getis%20first%20touch _asbp_gameinstance_showroom))
    ;[1 1 1] Set deepLevel on
    (bind _asbp_gameinstance_showroom_2 (Utilities|Casting|CastToBP_Gameinstance_showroom _returnvalue))
    (Variables|/Game/Showroom_Navigation/Gameinstance/BP_Gameinstance_showroom.BP_Gameinstance_showroom_C|SetIs_deep_Level _asbp_gameinstance_showroom_2 true)
    (bind _asbp_gameinstance_showroom_3 (Utilities|Casting|CastToBP_Gameinstance_showroom _returnvalue))
    ;[1 1 1] Get Transforms from Pawn
    (bind _asbp_focus_pawn_complex (Utilities|Casting|CastToBP_FocusPawnComplex (Game|Player|GetPlayerPawn 0)))
    ;[1 1 1] Save Transforms LevelSwitch
    (Variables|/Game/Showroom_Navigation/Gameinstance/BP_Gameinstance_showroom.BP_Gameinstance_showroom_C|SetGI_ArmLocation_LevelSwitch_DeepP _asbp_gameinstance_showroom_3 (Transformation|GetWorldLocation (Variables|/Game/Showroom_Navigation/Blueprint/FocusPoint_Complex/BP_FocusPawnComplex.BP_FocusPawnComplex_C|GetSpringArm _asbp_focus_pawn_complex)))
    (Variables|/Game/Showroom_Navigation/Gameinstance/BP_Gameinstance_showroom.BP_Gameinstance_showroom_C|SetGI_ArmLength_LevelSwitch_DeepP _asbp_gameinstance_showroom_3 (Variables|/Script/Engine.SpringArmComponent|GetTargetArmLength (Variables|/Game/Showroom_Navigation/Blueprint/FocusPoint_Complex/BP_FocusPawnComplex.BP_FocusPawnComplex_C|GetSpringArm _asbp_focus_pawn_complex)))
    (Variables|/Game/Showroom_Navigation/Gameinstance/BP_Gameinstance_showroom.BP_Gameinstance_showroom_C|SetGI_ArmRotation_LevelSwitch_DeepP _asbp_gameinstance_showroom_3 (Class|SpringArmComponent|GetTargetRotation (Variables|/Game/Showroom_Navigation/Blueprint/FocusPoint_Complex/BP_FocusPawnComplex.BP_FocusPawnComplex_C|GetSpringArm _asbp_focus_pawn_complex)))
    (Variables|/Game/Showroom_Navigation/Gameinstance/BP_Gameinstance_showroom.BP_Gameinstance_showroom_C|SetGI_DefaultSceneRoot_LevelSwitch_DeepP _asbp_gameinstance_showroom_3 (.location (Transformation|GetActorTransform _asbp_focus_pawn_complex)))
    ;[1 1 1] Open Level
    (Game|OpenLevel(byName) (Variables|Default|GetLevelToGo))))

(event EventBeginPlay
  ;[1 1 1] Set click Events
  (bind _asplayer_controller (Utilities|Casting|CastToPlayerController (Game|GetPlayerController 0)))
  (Variables|/Script/Engine.PlayerController|SetbEnableClickEvents _asplayer_controller true))

(event EventTick
  (params (DeltaSeconds :type Float%20%28single-precision%29))
  ;[1 1 1] Text_Labels - orient to Kamera
  (if (Variables|Default|GetShowLabels?)
    (Transformation|SetWorldRotation (Variables|Default|GetPivot) (Math|Rotator|FindLookatRotation (Transformation|GetActorLocation) (Transformation|GetActorLocation (Game|GetPlayerCameraManager 0))) false false)))

(fn ConstructionScript
  (bind _button_scale (Variables|Default|GetButton_Scale))
  (bind _only_text_size (Variables|Default|GetOnly_Text_Size))
  (bind _returnvalue (/ _button_scale 32.0))
  ;[1 1 1] Set Labels on/off
  (if (Variables|Default|GetShowLabels?)
    (Rendering|SetVisibility (Variables|Default|GetTextRender) true false)
    (Rendering|Components|TextRender|SetText (Variables|Default|GetTextRender) (Utilities|Text|ToText(String) (Variables|Default|GetLabelText)))
    (else
      (Rendering|SetVisibility (Variables|Default|GetTextRender) false false)))
  ;[1 1 1] Set Billboard transforms
  (Class|MaterialBillboardComponent|SetElements (Variables|Default|GetMaterialBillboard) (Utilities|Array|MakeArray (Utilities|Struct|MakeMaterialSpriteElement (Variables|Default|GetBillboard) 0 false _button_scale _button_scale)))
  (Transformation|SetRelativeScale3D (Variables|Default|GetPivot) (Math|Vector|MakeVector _returnvalue _returnvalue _returnvalue))
  (Transformation|SetRelativeScale3D (Variables|Default|GetText_Size) (Math|Vector|MakeVector _only_text_size _only_text_size _only_text_size)))