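; BP_BaseFocusTarget is a showroom navigation focus point, an actor with a spring arm and camera that define a view.
; Its construction script sets the arm length and relative rotation from its own variables and copies the field of view from the BP_FocusPawnComplex found in the level.
; It also resets the root's world rotation to zero, so rotating the placed actor has no effect.
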(event EventBeginPlay)

(fn ConstructionScript
  ;[1 1 1] Set Base Springarm
  (Variables|/Script/Engine.SpringArmComponent|SetTargetArmLength (Variables|Default|GetSpringArm) (Variables|Default|GetBasePointArmLength))
  (Transformation|SetRelativeRotation (Variables|Default|GetSpringArm) (Variables|Default|GetCamera%20Rotation) false false)
  ;[1 1 1] Set FOV from Pawn
  (bind _returnvalue (Actor|GetActorOfClass "/Game/Showroom_Navigation/Blueprint/FocusPoint_Complex/BP_FocusPawnComplex.BP_FocusPawnComplex_C"))
  (Camera|SetFieldOfView (Variables|Default|GetCamera) (Variables|/Game/Showroom_Navigation/Blueprint/FocusPoint_Complex/BP_FocusPawnComplex.BP_FocusPawnComplex_C|GetField_of_View _returnvalue))
  ;[1 1 1] Block Rotation on Root
  (Transformation|SetWorldRotation (Variables|Default|GetDefaultSceneRoot) "0, 0, 0" false false))