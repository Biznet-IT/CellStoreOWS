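; BP_BaseTarget is a showroom navigation camera target that provides a viewpoint and a tour button label.
; Its construction script configures the spring arm, copies field of view from BP_MasterPawn and zeroes root world rotation.
; It also writes its arm length to the showroom GameInstance for level switching.
; TourButtonLabels returns a custom tour name when enabled, otherwise the display name stripped of base, zoom and waypoint target prefixes.
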(event EventBeginPlay)

(fn ConstructionScript
  ;[1 1 1] Setup camera
  (Variables|/Script/Engine.SpringArmComponent|SetTargetArmLength (Variables|Default|GetSpringArm) (Variables|Default|GetBasePointArmLength))
  (Transformation|SetRelativeRotation (Variables|Default|GetSpringArm) (Variables|Default|GetCamera%20Rotation) false false)
  ;[1 1 1] Set FOV from Pawn
  (bind _returnvalue (Actor|GetActorOfClass "/Game/Showroom_Navigation/Blueprint/BP_MasterPawn.BP_MasterPawn_C"))
  (Camera|SetFieldOfView (Variables|Default|GetCamera) (Variables|/Game/Showroom_Navigation/Blueprint/BP_MasterPawn.BP_MasterPawn_C|GetField_of_View _returnvalue))
  ;[1 1 1] Lock Root rotation
  (Transformation|SetWorldRotation (Variables|Default|GetDefaultSceneRoot) "0, 0, 0" false false)
  ;[1 1 1] Set Armlength Levelswitch
  (bind _asbp_gameinstance_showroom (Utilities|Casting|CastToBP_Gameinstance_showroom (Game|GetGameInstance)))
  (Variables|/Game/Showroom_Navigation/Gameinstance/BP_Gameinstance_showroom.BP_Gameinstance_showroom_C|SetGI_ArmLength_LevelSwitch _asbp_gameinstance_showroom (Variables|Default|GetBasePointArmLength)))

(fn TourButtonLabels
  (if (Variables|Default|GetActivate%20Tour%20Name)
    ;[1 1 1] TourNames_EnterName Dialog
    (return (Variables|Default|GetTour%20Name))
    (else
      ;[1 1 1] Tour Names Enter Display Names
      (return (Utilities|Text|ToText(String) (Utilities|String|Replace (Utilities|String|Replace (Utilities|String|Replace (Utilities|String|ToString(Text) (Utilities|Text|ToText(String) (Utilities|GetDisplayName self))) "BP_ZoomTarget") "BP_BaseTarget") "BP_WaypointTarget"))))))