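; BP_InfoPointBillboard01 is a showroom info point: a billboard button that adds a configurable widget to the viewport when touched or clicked.
; BeginPlay enables click events on the player controller, and the Box click and actor touch share one widget-creation path.
; The construction script applies label text, billboard material and scale settings.
; Tick toggles label visibility and, while shown, rotates the Cube to face the camera.
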(event OnClicked(Box)
  (params (TouchedComponent :type Primitive%20Component%20Object%20Reference) (ButtonPressed :type Key%20Structure))
  (bind _returnvalue (UserInterface|CreateWidget (Variables|Default|GetWidget_to_use) (Game|GetPlayerController 0)))
  (UserInterface|Viewport|AddtoViewport _returnvalue 0))

(event EventBeginPlay
  (bind _asplayer_controller (Utilities|Casting|CastToPlayerController (Game|GetPlayerController 0)))
  (Variables|/Script/Engine.PlayerController|SetbEnableClickEvents _asplayer_controller true))

(event EventTick
  (params (DeltaSeconds :type Float%20%28single-precision%29))
  ;[1 1 1] Text_Labels
  (if (Variables|Default|GetShowLabels?)
    (Rendering|SetVisibility (Variables|Default|GetTextRender) true false)
    (Transformation|SetWorldRotation (Variables|Default|GetCube) (Math|Rotator|FindLookatRotation (Transformation|GetActorLocation) (Transformation|GetActorLocation (Game|GetPlayerCameraManager 0))) false false)
    (else
      (Rendering|SetVisibility (Variables|Default|GetTextRender) false false))))

(event EventActorOnInputTouchBegin
  (params (FingerIndex :type ETouchIndex%20Enum :default "Touch1"))
  (bind _returnvalue (UserInterface|CreateWidget (Variables|Default|GetWidget_to_use) (Game|GetPlayerController 0)))
  (UserInterface|Viewport|AddtoViewport _returnvalue 0))

(fn ConstructionScript
  (bind _button_scale (Variables|Default|GetButton_Scale))
  (bind _only_text_size (Variables|Default|GetOnly_Text_Size))
  (bind _returnvalue (/ _button_scale 32.0))
  (Rendering|Components|TextRender|SetText (Variables|Default|GetTextRender) (Utilities|Text|ToText(String) (Variables|Default|GetLabelText)))
  (Class|MaterialBillboardComponent|SetElements (Variables|Default|GetMaterialBillboard) (Utilities|Array|MakeArray (Utilities|Struct|MakeMaterialSpriteElement (Variables|Default|GetBillboard) 0 false _button_scale _button_scale)))
  (Transformation|SetRelativeScale3D (Variables|Default|GetCube) (Math|Vector|MakeVector _returnvalue _returnvalue _returnvalue))
  (Transformation|SetRelativeScale3D (Variables|Default|GetText_Size) (Math|Vector|MakeVector _only_text_size _only_text_size _only_text_size)))