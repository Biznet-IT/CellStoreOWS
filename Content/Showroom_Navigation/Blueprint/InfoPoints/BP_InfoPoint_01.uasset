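; BP_InfoPoint_01 is a clickable info point actor in the showroom navigation set that opens a UI widget.
; A click or touch on Info_collider creates the WidgetToUse widget for player 0 and adds it to the viewport.
; Cursor hover over the collider swaps the InfopointIcon and InfopointIconOn components' visibility to show a highlighted state.
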(event OnClicked(Info_collider)
  (params (TouchedComponent :type Primitive%20Component%20Object%20Reference) (ButtonPressed :type Key%20Structure))
  (bind _returnvalue (UserInterface|CreateWidget (Variables|Default|GetWidget_to_Use) (Game|GetPlayerController 0)))
  (UserInterface|Viewport|AddtoViewport _returnvalue 0))

(event OnInputTouchBegin(Info_collider)
  (params (FingerIndex :type ETouchIndex%20Enum :default "Touch1") (TouchedComponent :type Primitive%20Component%20Object%20Reference))
  (bind _returnvalue (UserInterface|CreateWidget (Variables|Default|GetWidget_to_Use) (Game|GetPlayerController 0)))
  (UserInterface|Viewport|AddtoViewport _returnvalue 0))

(event OnEndCursorOver(Info_collider)
  (params (TouchedComponent :type Primitive%20Component%20Object%20Reference))
  (Rendering|SetVisibility (Variables|Default|GetInfopoint_Icon) true false)
  (Rendering|SetVisibility (Variables|Default|GetInfopoint_Icon_on) false false))

(event OnBeginCursorOver(Info_collider)
  (params (TouchedComponent :type Primitive%20Component%20Object%20Reference))
  (Rendering|SetVisibility (Variables|Default|GetInfopoint_Icon) false false)
  (Rendering|SetVisibility (Variables|Default|GetInfopoint_Icon_on) true false))

(fn ConstructionScript)