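; Showroom hotspot actor that opens a target level when its trigger box is clicked or tapped, ignoring taps during touch movement.
; Before travel it clears the tour widget array and saves first-person transform and rotation, or orbit pawn spring-arm state, to the GameInstance.
; The construction script sizes the billboard, trigger and optional text label.
; On Tick, enabled labels turn toward the camera.
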(event OnInputTouchEnd(Box_Trigger)
  (params (FingerIndex :type ETouchIndex%20Enum :default "Touch1") (TouchedComponent :type Primitive%20Component%20Object%20Reference))
  ;[1 1 1] Do not open when Touch is moving
  (bind _asbp_gameinstance_showroom (Utilities|Casting|CastToBP_Gameinstance_showroom (Game|GetGameInstance)))
  (if (not (Variables|/Game/Showroom_Navigation/Gameinstance/BP_Gameinstance_showroom.BP_Gameinstance_showroom_C|Getis_Touch_moving _asbp_gameinstance_showroom))
    ;[1 1 1] Clear_Timeline_WidgetArray
    (bind _asbp_gameinstance_showroom_2 (Utilities|Casting|CastToBP_Gameinstance_showroom (Game|GetGameInstance)))
    (Utilities|Array|Clear (Variables|/Game/Showroom_Navigation/Gameinstance/BP_Gameinstance_showroom.BP_Gameinstance_showroom_C|GetGI_TourWidgetArray _asbp_gameinstance_showroom_2))
    ;[1 1 1] Is FPS?
    (if (Variables|/Game/Showroom_Navigation/Gameinstance/BP_Gameinstance_showroom.BP_Gameinstance_showroom_C|GetFPS_ON _asbp_gameinstance_showroom_2)
      ;[1 1 1] Save_First_Person_Transforms
      (bind _asbp_gameinstance_showroom_3 (Utilities|Casting|CastToBP_Gameinstance_showroom (Game|GetGameInstance)))
      (bind _asbp_first_person_character (Utilities|Casting|CastToBP_FirstPersonCharacter (Game|GetPlayerCharacter 0)))
      (Variables|/Game/Showroom_Navigation/Gameinstance/BP_Gameinstance_showroom.BP_Gameinstance_showroom_C|Setcontroler_rotation _asbp_gameinstance_showroom_3 (Pawn|GetControlRotation _asbp_first_person_character :!class /Script/Engine.Pawn))
      (Variables|/Game/Showroom_Navigation/Gameinstance/BP_Gameinstance_showroom.BP_Gameinstance_showroom_C|SetPlayertransform _asbp_gameinstance_showroom_3 (Transformation|GetActorTransform _asbp_first_person_character))
      (else
        (bind _asbp_gameinstance_showroom_4 (Utilities|Casting|CastToBP_Gameinstance_showroom (Game|GetGameInstance)))
        ;[1 1 1] Get transform from Pawn
        (bind _asbp_master_pawn (Utilities|Casting|CastToBP_MasterPawn (Game|Player|GetPlayerPawn 0)))
        ;[1 1 1] Save_Pawn_Transform - Levelswitch
        (Variables|/Game/Showroom_Navigation/Gameinstance/BP_Gameinstance_showroom.BP_Gameinstance_showroom_C|SetGI_ArmLocation_LevelSwitch _asbp_gameinstance_showroom_4 (Transformation|GetWorldLocation (Variables|/Game/Showroom_Navigation/Blueprint/BP_MasterPawn.BP_MasterPawn_C|GetSpringArm _asbp_master_pawn)))
        (Variables|/Game/Showroom_Navigation/Gameinstance/BP_Gameinstance_showroom.BP_Gameinstance_showroom_C|SetGI_ArmLength_LevelSwitch _asbp_gameinstance_showroom_4 (Variables|/Script/Engine.SpringArmComponent|GetTargetArmLength (Variables|/Game/Showroom_Navigation/Blueprint/BP_MasterPawn.BP_MasterPawn_C|GetSpringArm _asbp_master_pawn)))
        (Variables|/Game/Showroom_Navigation/Gameinstance/BP_Gameinstance_showroom.BP_Gameinstance_showroom_C|SetGI_ArmRotation_LevelSwitch _asbp_gameinstance_showroom_4 (Class|SpringArmComponent|GetTargetRotation (Variables|/Game/Showroom_Navigation/Blueprint/BP_MasterPawn.BP_MasterPawn_C|GetSpringArm _asbp_master_pawn)))
        (Variables|/Game/Showroom_Navigation/Gameinstance/BP_Gameinstance_showroom.BP_Gameinstance_showroom_C|SetGI_DefaultSceneRoot_LevelSwitch _asbp_gameinstance_showroom_4 (.location (Transformation|GetActorTransform _asbp_master_pawn)))))
    ;[1 1 1] open level
    (Game|OpenLevel(byName) (Variables|Default|GetLevelToGo))))

(event OnClicked(Box_Trigger)
  (params (TouchedComponent :type Primitive%20Component%20Object%20Reference) (ButtonPressed :type Key%20Structure))
  ;[1 1 1] Do not open when Touch is moving
  (bind _asbp_gameinstance_showroom (Utilities|Casting|CastToBP_Gameinstance_showroom (Game|GetGameInstance)))
  (if (not (Variables|/Game/Showroom_Navigation/Gameinstance/BP_Gameinstance_showroom.BP_Gameinstance_showroom_C|Getis%20first%20touch _asbp_gameinstance_showroom))
    ;[1 1 1] Clear_Timeline_WidgetArray
    (bind _asbp_gameinstance_showroom_2 (Utilities|Casting|CastToBP_Gameinstance_showroom (Game|GetGameInstance)))
    (Utilities|Array|Clear (Variables|/Game/Showroom_Navigation/Gameinstance/BP_Gameinstance_showroom.BP_Gameinstance_showroom_C|GetGI_TourWidgetArray _asbp_gameinstance_showroom_2))
    ;[1 1 1] Is FPS?
    (if (Variables|/Game/Showroom_Navigation/Gameinstance/BP_Gameinstance_showroom.BP_Gameinstance_showroom_C|GetFPS_ON _asbp_gameinstance_showroom_2)
      ;[1 1 1] Save_First_Person_Transforms
      (bind _asbp_gameinstance_showroom_3 (Utilities|Casting|CastToBP_Gameinstance_showroom (Game|GetGameInstance)))
      (bind _asbp_first_person_character (Utilities|Casting|CastToBP_FirstPersonCharacter (Game|GetPlayerCharacter 0)))
      (Variables|/Game/Showroom_Navigation/Gameinstance/BP_Gameinstance_showroom.BP_Gameinstance_showroom_C|Setcontroler_rotation _asbp_gameinstance_showroom_3 (Pawn|GetControlRotation _asbp_first_person_character :!class /Script/Engine.Pawn))
      (Variables|/Game/Showroom_Navigation/Gameinstance/BP_Gameinstance_showroom.BP_Gameinstance_showroom_C|SetPlayertransform _asbp_gameinstance_showroom_3 (Transformation|GetActorTransform _asbp_first_person_character))
      (else
        (bind _asbp_gameinstance_showroom_4 (Utilities|Casting|CastToBP_Gameinstance_showroom (Game|GetGameInstance)))
        ;[1 1 1] Get transform from Pawn
        (bind _asbp_master_pawn (Utilities|Casting|CastToBP_MasterPawn (Game|Player|GetPlayerPawn 0)))
        ;[1 1 1] Save_Pawn_Transform - Levelswitch
        (Variables|/Game/Showroom_Navigation/Gameinstance/BP_Gameinstance_showroom.BP_Gameinstance_showroom_C|SetGI_ArmLocation_LevelSwitch _asbp_gameinstance_showroom_4 (Transformation|GetWorldLocation (Variables|/Game/Showroom_Navigation/Blueprint/BP_MasterPawn.BP_MasterPawn_C|GetSpringArm _asbp_master_pawn)))
        (Variables|/Game/Showroom_Navigation/Gameinstance/BP_Gameinstance_showroom.BP_Gameinstance_showroom_C|SetGI_ArmLength_LevelSwitch _asbp_gameinstance_showroom_4 (Variables|/Script/Engine.SpringArmComponent|GetTargetArmLength (Variables|/Game/Showroom_Navigation/Blueprint/BP_MasterPawn.BP_MasterPawn_C|GetSpringArm _asbp_master_pawn)))
        (Variables|/Game/Showroom_Navigation/Gameinstance/BP_Gameinstance_showroom.BP_Gameinstance_showroom_C|SetGI_ArmRotation_LevelSwitch _asbp_gameinstance_showroom_4 (Class|SpringArmComponent|GetTargetRotation (Variables|/Game/Showroom_Navigation/Blueprint/BP_MasterPawn.BP_MasterPawn_C|GetSpringArm _asbp_master_pawn)))
        (Variables|/Game/Showroom_Navigation/Gameinstance/BP_Gameinstance_showroom.BP_Gameinstance_showroom_C|SetGI_DefaultSceneRoot_LevelSwitch _asbp_gameinstance_showroom_4 (.location (Transformation|GetActorTransform _asbp_master_pawn)))))
    ;[1 1 1] open level
    (Game|OpenLevel(byName) (Variables|Default|GetLevelToGo))))

(event EventBeginPlay
  ;[1 1 1] enable click
  (bind _asplayer_controller (Utilities|Casting|CastToPlayerController (Game|GetPlayerController 0)))
  (Variables|/Script/Engine.PlayerController|SetbEnableClickEvents _asplayer_controller true))

(event EventTick
  (params (DeltaSeconds :type Float%20%28single-precision%29))
  ;[1 1 1] Text_Labels
  (if (Variables|Default|GetShowLabels?)
    (Transformation|SetWorldRotation (Variables|Default|GetPivot) (Math|Rotator|FindLookatRotation (Transformation|GetActorLocation) (Transformation|GetActorLocation (Game|GetPlayerCameraManager 0))) false false)))

(fn ConstructionScript
  (bind _button_scale (Variables|Default|GetButton_Scale))
  (bind _only_text_size (Variables|Default|GetOnly_Text_Size))
  (bind _returnvalue (/ _button_scale 32.0))
  ;[1 1 1] Show Labels?
  (if (Variables|Default|GetShowLabels?)
    (Rendering|SetVisibility (Variables|Default|GetTextRender) true false)
    (Rendering|Components|TextRender|SetText (Variables|Default|GetTextRender) (Utilities|Text|ToText(String) (Variables|Default|GetLabelText)))
    (else
      (Rendering|SetVisibility (Variables|Default|GetTextRender) false false)))
  ;[1 1 1] Set Billboard and Transforms
  (Class|MaterialBillboardComponent|SetElements (Variables|Default|GetMaterialBillboard) (Utilities|Array|MakeArray (Utilities|Struct|MakeMaterialSpriteElement (Variables|Default|GetBillboard) 0 false _button_scale _button_scale)))
  (Transformation|SetRelativeScale3D (Variables|Default|GetPivot) (Math|Vector|MakeVector _returnvalue _returnvalue _returnvalue))
  (Transformation|SetRelativeScale3D (Variables|Default|GetText_Size) (Math|Vector|MakeVector _only_text_size _only_text_size _only_text_size)))