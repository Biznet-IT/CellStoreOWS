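; Farm mill prop that is either a wooden water mill or a windmill and spins while the game runs.
; The construction script swaps the mill mesh by a clamped type, showing the axle with collision only for the water mill.
; It also stretches the axle along Z by a rounded, clamped length.
; On BeginPlay a timeline drives the mill mesh's relative pitch, scaled by Speed.
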(event EventBeginPlay
  (bind _rotation (Timeline|Timeline_0 Play)
    (:Update
      (Transformation|SetRelativeRotation (Variables|Default|GetMill_Mesh) (Math|Rotator|MakeRotator 0.0 (* (* _rotation -3.6e+02) (Variables|Default|GetSpeed)) 0.0) false false))))

(fn ConstructionScript
  (Variables|Default|SetAxeLength (Math|Float|Clamp(Float) (/ (Math|Conversions|ToFloat(Integer) (Math|Float|Round (* (Variables|Default|GetAxeLength) 1e+01))) 1e+01) 1.0 5.0))
  (Transformation|SetWorldScale3D (Variables|Default|GetMill_Axe_Mesh) (Math|Vector|MakeVector 1.0 1.0 (Variables|Default|GetAxeLength)))
  (bind _output_get (Variables|Default|SetMillType (Math|Integer|Clamp(Integer) (Variables|Default|GetMillType) 0 1)))
  (switch int _output_get
    (:0
      (Components|StaticMesh|SetStaticMesh (Variables|Default|GetMill_Mesh) "/Game/Medieval_Environment/Medieval_Build_Vol1/Meshes/SM_MF_Wood_WaterMill_01.SM_MF_Wood_WaterMill_01")
      (Rendering|SetVisibility (Variables|Default|GetMill_Axe_Mesh) true false)
      (Collision|SetCollisionEnabled (Variables|Default|GetMill_Axe_Mesh) "QueryAndPhysics"))
    (:1
      (Components|StaticMesh|SetStaticMesh (Variables|Default|GetMill_Mesh) "/Game/Medieval_Environment/Medieval_Build_Vol1/Meshes/SM_MF_Wood_WindMill_01.SM_MF_Wood_WindMill_01")
      (Rendering|SetVisibility (Variables|Default|GetMill_Axe_Mesh) false false)
      (Collision|SetCollisionEnabled (Variables|Default|GetMill_Axe_Mesh) "NoCollision"))))