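; Medieval farm door Blueprint that swings open when something overlaps its Sphere component and closes when the overlap ends.
; The overlap events play and reverse a timeline, whose curve scales the yaw of the DoorLeft mesh relative to its parent.
; The construction script clamps DoorType and uses it to pick the small or big wooden door mesh.
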(event OnComponentBeginOverlap(Sphere)
  (params (OverlappedComponent :type Primitive%20Component%20Object%20Reference) (OtherActor :type Actor%20Object%20Reference) (OtherComp :type Primitive%20Component%20Object%20Reference) (OtherBodyIndex :type Integer) (bFromSweep :type Boolean) (SweepResult :type Hit%20Result%20Structure%20%28by%20ref%29))
  (bind _rotationcoeff (Timeline|Timeline_Rotation Play)
    (:Update
      (Transformation|SetRelativeRotation (Variables|Default|GetDoor_Left) (Math|Rotator|MakeRotator 0.0 0.0 (* _rotationcoeff 85.0)) false false))))

(event OnComponentEndOverlap(Sphere)
  (params (OverlappedComponent :type Primitive%20Component%20Object%20Reference) (OtherActor :type Actor%20Object%20Reference) (OtherComp :type Primitive%20Component%20Object%20Reference) (OtherBodyIndex :type Integer))
  (bind _rotationcoeff (Timeline|Timeline_Rotation Reverse)
    (:Update
      (Transformation|SetRelativeRotation (Variables|Default|GetDoor_Left) (Math|Rotator|MakeRotator 0.0 0.0 (* _rotationcoeff 85.0)) false false))))

(fn ConstructionScript
  (bind _output_get (Variables|Default|SetDoorType (Math|Integer|Clamp(Integer) (Variables|Default|GetDoorType) 0 1)))
  (switch int _output_get
    (:0
      (Components|StaticMesh|SetStaticMesh (Variables|Default|GetDoor_Left) "/Game/Medieval_Environment/Medieval_Build_Vol1/Meshes/SM_MF_Wood_Door_Small_01.SM_MF_Wood_Door_Small_01"))
    (:1
      (Components|StaticMesh|SetStaticMesh (Variables|Default|GetDoor_Left) "/Game/Medieval_Environment/Medieval_Build_Vol1/Meshes/SM_MF_Wood_Door_Big_01.SM_MF_Wood_Door_Big_01"))))