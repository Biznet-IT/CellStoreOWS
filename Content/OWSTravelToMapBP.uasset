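; OWS map-travel trigger volume that moves an overlapping player character to another zone's map server.
; On server overlap it flags the transfer, optionally shows loading and freezes movement, then requests the least-populated map server.
; The reply saves player data and travels to a fixed or axis-offset spawn, with optional floor trace and relative rotation.
; Lookup errors restore walking, hide loading and clear the flag; the travel step is marked not production ready.
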(event OnComponentBeginOverlap(Box)
  (params (OverlappedComponent :type Primitive%20Component%20Object%20Reference) (OtherActor :type Actor%20Object%20Reference) (OtherComp :type Primitive%20Component%20Object%20Reference) (OtherBodyIndex :type Integer) (bFromSweep :type Boolean) (SweepResult :type Hit%20Result%20Structure%20%28by%20ref%29))
  (bind _returnvalue (Transformation|GetActorLocation))
  (bind (_x _y _z) (Math|Vector|BreakVector _returnvalue))
  ;[1 1 1] Build needed references, if any of these fail don't bother going any further into the process as they are needed later
  (Networking|SwitchHasAuthority
    (:Authority
      (bind _asowscharacter (Utilities|Casting|CastToOWSCharacter OtherActor)
        (:then
          (bind _output_get (Variables|Default|SetCharacterReference _asowscharacter))
          (bind _asowsplayer_controller (Utilities|Casting|CastToOWSPlayerController (Pawn|GetController _output_get))
            (:then
              (bind _output_get_2 (Variables|Default|SetPlayerControllerReference _asowsplayer_controller))
              (bind _asowsplayer_state (Utilities|Casting|CastToOWSPlayerState (Variables|/Script/Engine.Controller|GetPlayerState _output_get_2))
                (:then
                  (Variables|Default|SetPlayerStateReference _asowsplayer_state)
                  ;[1 1 1] SERVER - When a player overlaps with boundary and they are not already attempting to travel try to initiate one.
                  (if (not (Variables|/Script/OWSPlugin.OWSCharacter|GetIsTransferringBetweenMaps _output_get))
                    (if (Utilities|Enum|NotEqual(Enum) (Variables|Default|GetZoneName) "")
                      (Variables|/Script/OWSPlugin.OWSCharacter|SetIsTransferringBetweenMaps (Variables|Default|GetCharacterReference) true)
                      (if (Variables|Default|GetUseDynamicSpawnLocation)
                        ;[1 1 1] Determine the dynamic spawn axis and set the appropriate offset.
                        (Variables|Default|SetZAxisOffset (- (.Z (Math|Vector|BreakVector (Transformation|GetActorLocation _output_get))) _z))
                        (switch Utilities|FlowControl|Switch|SwitchonDynamicAxisType (Variables|Default|GetDynamicSpawnAxis)
                          (:XAxis
                            (Variables|Default|SetAxisOffset (- _x (.X (Math|Vector|BreakVector (Transformation|GetActorLocation _output_get))))))
                          (:YAxis
                            (Variables|Default|SetAxisOffset (- _y (.Y (Math|Vector|BreakVector (Transformation|GetActorLocation _output_get))))))))
                      ;[1 1 1] Show loading screen, disable Character  Movement and try to Travel to Map
                      (if (Variables|Default|GetShowLoadingDialog)
                        (Default|CallShowLoadingDialogEvent (PlayerState|GetPlayerName (Variables|/Script/Engine.Pawn|GetPlayerState (Pawn|GetControlledPawn (Variables|Default|GetPlayerControllerReference)))))
                        (Pawn|Components|CharacterMovement|DisableMovement (Variables|/Script/Engine.Character|GetCharacterMovement (Variables|Default|GetCharacterReference))))
                      (Class|OWSTraveltoMapActor|GetMapServertoTravelto (Variables|Default|GetPlayerControllerReference) "MapWithFewestPlayers")
                      (Development|PrintString "Get Map Server to Travel To Called!")
                      (else
                        (Development|PrintString "Empty Zone Name!")))
                    (else
                      (Development|PrintString "Already transferring!"))))
                (:CastFailed
                  (Development|PrintString "Cast Failed (OWSPlayerState)!"))))
            (:CastFailed
              (Development|PrintString "Cast Failed (OWSPlayerController)!"))))
        (:CastFailed
          (Development|PrintString "Cast Failed (OWSCharacter)!"))))))

(event OnComponentEndOverlap(Box)
  (params (OverlappedComponent :type Primitive%20Component%20Object%20Reference) (OtherActor :type Actor%20Object%20Reference) (OtherComp :type Primitive%20Component%20Object%20Reference) (OtherBodyIndex :type Integer))
  ;[1 1 1] Disconnected
  (Networking|SwitchHasAuthority
    (:Authority
      (bind _asowscharacter (Utilities|Casting|CastToOWSCharacter OtherActor))
      (Utilities|FlowControl|Delay 5.0)
      (Utilities|IsValid _asowscharacter
        (:Is%20Valid
          (Variables|/Script/OWSPlugin.OWSCharacter|SetIsTransferringBetweenMaps _asowscharacter false))))))

(event EventNotifyMapServertoTravelto
  (params (ServerAndPort :type String))
  (bind _invertdynamicaxisoffset (Variables|Default|GetInvertDynamicAxisOffset))
  (bind _startingrotation (Variables|Default|GetStartingRotation))
  (bind _usedynamicspawnrotation (Variables|Default|GetUseDynamicSpawnRotation))
  (bind _dynamicspawnrotationoffeset (Variables|Default|GetDynamicSpawnRotationOffeset))
  (bind _playercontrollerreference (Variables|Default|GetPlayerControllerReference))
  (bind _characterreference (Variables|Default|GetCharacterReference))
  (bind _locationonmap (Variables|Default|GetLocationOnMap))
  (bind _zaxisoffset (Variables|Default|GetZAxisOffset))
  (bind _axisoffset (Variables|Default|GetAxisOffset))
  (bind (_roll _pitch _yaw) (Math|Rotator|BreakRotator _dynamicspawnrotationoffeset))
  (bind _returnvalue (- 0.0 _axisoffset))
  (bind (_x _y _z) (Math|Vector|BreakVector _locationonmap))
  (bind _returnvalue_2 (Transformation|GetActorRotation _characterreference))
  (bind (_roll_2 _pitch_2 _yaw_2) (Math|Rotator|BreakRotator _returnvalue_2))
  (bind _returnvalue_3 (+ _z _zaxisoffset))
  (bind _returnvalue_4 (select _invertdynamicaxisoffset _axisoffset _returnvalue))
  (bind _returnvalue_5 (+ _roll _roll_2))
  (bind _returnvalue_6 (+ _yaw _yaw_2))
  (bind _returnvalue_7 (+ _pitch _pitch_2))
  (bind _returnvalue_8 (Math|Rotator|MakeRotator _returnvalue_5 _returnvalue_7 _returnvalue_6))
  (bind _returnvalue_9 (select _usedynamicspawnrotation _returnvalue_8 _startingrotation))
  (bind (_roll_3 _pitch_3 _yaw_3) (Math|Rotator|BreakRotator _returnvalue_9))
  ;[1 1 1] SERVER - We got a map/server to travel to, so build a string to send with the travel to map function.  (This is NOT production ready)
  (Development|PrintString "Notify Map Server to Travel To")
  (if (Variables|Default|GetUseDynamicSpawnLocation)
    ;;[1 1 1] Build the appropriate point to move for the string function below
    (switch Utilities|FlowControl|Switch|SwitchonDynamicAxisType (Variables|Default|GetDynamicSpawnAxis)
      (:XAxis
        (Variables|Default|SetPointToMoveTo (Math|Vector|MakeVector (+ _x _returnvalue_4) _y _returnvalue_3)))
      (:YAxis
        (Variables|Default|SetPointToMoveTo (Math|Vector|MakeVector _x (+ _y _returnvalue_4) _returnvalue_3))))
    (else
      (Variables|Default|SetPointToMoveTo (Variables|Default|GetLocationOnMap))))
  (bind _outhit (Collision|LineTraceForObjects (+ (Variables|Default|GetPointToMoveTo) "0, 0,100000.000000") (+ (Variables|Default|GetPointToMoveTo) "0, 0,-100000.000000") (Utilities|Array|MakeArray "ObjectTypeQuery1") false 0 "None"))
  (Variables|Default|SetPointToMoveTo (Math|Vector|MakeVector (.x (Variables|Default|GetPointToMoveTo)) (.y (Variables|Default|GetPointToMoveTo)) (select (Variables|Default|GetUseLineTraceToFindFloor) (+ (.Z (Math|Vector|BreakVector (.Location (Collision|BreakHitResult _outhit)))) 1e+01) (.z (Variables|Default|GetPointToMoveTo)))))
  ;;[1 1 1] Save the player and initiate the Travel command
  (Class|OWSPlayerController|SaveAllPlayerData _playercontrollerreference)
  (Class|OWSPlayerController|TraveltoMap2 _playercontrollerreference ServerAndPort (.X (Math|Vector|BreakVector (Variables|Default|GetPointToMoveTo))) (.Y (Math|Vector|BreakVector (Variables|Default|GetPointToMoveTo))) (+ (.Z (Math|Vector|BreakVector (Variables|Default|GetPointToMoveTo))) 5.0) _roll_3 _pitch_3 _yaw_3 (PlayerState|GetPlayerName (Variables|Default|GetPlayerStateReference)) false)
  (Development|PrintString "Called Travl to Map!"))

(event EventErrorMapServertoTravelto
  (params (ErrorMsg :type String))
  ;[1 1 1] If there is an error finding a map to travel to show the error message, unlock movement and remove loading screen
  (Development|PrintString ErrorMsg)
  (Pawn|Components|CharacterMovement|SetMovementMode (Variables|/Script/Engine.Character|GetCharacterMovement (Variables|Default|GetCharacterReference)) "MOVE_Walking" 0)
  (Default|CallHideLoadingDialogEvent (PlayerState|GetPlayerName (Variables|/Script/Engine.Pawn|GetPlayerState (Pawn|GetControlledPawn (Variables|Default|GetPlayerControllerReference)))))
  (Variables|/Script/OWSPlugin.OWSCharacter|SetIsTransferringBetweenMaps (Variables|Default|GetCharacterReference) false))

(fn ConstructionScript)